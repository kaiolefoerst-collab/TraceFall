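; Player character Blueprint that provides basic walk and turn controls through Enhanced Input.
; On possession it stops any movement and adds the IMC_PlayerCharacter mapping context to the player's input subsystem.
; IA_Walk drives movement along the actor's forward vector and prints the last input vector for debugging.
; IA_Turn applies scaled controller yaw.
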(event `EnhancedInput|/Game/Input/IA_Walk`
  (params (ActionValue :type "Float (double-precision)") (ElapsedSeconds :type "Float (double-precision)") (TriggeredSeconds :type "Float (double-precision)") (InputAction :type "InputAction Object Reference" :default "/Game/Input/IA_Walk.IA_Walk"))
  (:`Triggered`
    (`self.AddMovementInput` (* ActionValue (`self.GetActorForwardVector`)))
    (`KismetSystemLibrary.PrintString` (`KismetStringLibrary.Conv_VectorToString` (`self.GetLastMovementInputVector`)))))

(event `EnhancedInput|/Game/Input/IA_Turn`
  (params (ActionValue :type "Float (double-precision)") (ElapsedSeconds :type "Float (double-precision)") (TriggeredSeconds :type "Float (double-precision)") (InputAction :type "InputAction Object Reference" :default "/Game/Input/IA_Turn.IA_Turn"))
  (:`Triggered`
    (`self.AddControllerYawInput` (* ActionValue 2.0))))

(event `self.ReceivePossessed`
  (params (NewController :type "Controller Object Reference"))
  (`MovementComponent.StopMovementImmediately` (`self.CharacterMovement`))
  (bind _returnvalue (`InputDeviceLibrary.GetPlayerControllerFromInputDevice` (struct)))
  (`EnhancedInputSubsystemInterface.AddMappingContext` (pcsubsystem `EnhancedInputLocalPlayerSubsystem` _returnvalue) "/Game/Input/IMC_PlayerCharacter.IMC_PlayerCharacter" 0 (struct)))

(event `self.ReceiveTick`
  (params (DeltaSeconds :type "Float (single-precision)")))

(event `self.ReceiveBeginPlay`)

(fn `UserConstructionScript`)