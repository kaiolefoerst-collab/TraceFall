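; Pilotable spaceship pawn that the player controller possesses when anything overlaps its cockpit trigger, swapping the character's input mapping for the spaceship's.
; Move input drives forward movement and a target yaw speed, which Tick eases with FInterpTo for smoothed turning.
; Exit input teleports the player character to the exit point and possesses it again.
; BeginPlay also adds the spaceship mapping and shows an interaction hint widget.
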(event `EnhancedInput|/Game/Input/IA_Spaceship_ExitCockpit`
  (params (ActionValue :type Boolean) (ElapsedSeconds :type "Float (double-precision)") (TriggeredSeconds :type "Float (double-precision)") (InputAction :type "InputAction Object Reference" :default "/Game/Input/IA_Spaceship_ExitCockpit.IA_Spaceship_ExitCockpit"))
  (:`Triggered`
    (bind _returnvalue (`InputDeviceLibrary.GetPlayerControllerFromInputDevice` (struct)))
    (`self.K2_SetActorTransform` (`self.PlayerCharacter`) (`SceneComponent.K2_GetComponentToWorld` (`self.PlayerExitPoint`)) false true)
    (`Controller.Possess` _returnvalue (`self.PlayerCharacter`))))

(event `EnhancedInput|/Game/Input/IA_Move`
  (params (ActionValue :type "Vector2D Structure") (ElapsedSeconds :type "Float (double-precision)") (TriggeredSeconds :type "Float (double-precision)") (InputAction :type "InputAction Object Reference" :default "/Game/Input/IA_Move.IA_Move"))
  (bind (_x _y) (`KismetMathLibrary.BreakVector2D` ActionValue))
  (:`Triggered`
    (set `self.TargetYawSpeed` (* _x 30.0))
    (`self.AddMovementInput` (`self.GetActorForwardVector`) _y))
  (:`Completed`
    (set `self.TargetYawSpeed` 0.0)))

(event `self.ReceiveTick`
  (params (DeltaSeconds :type "Float (single-precision)"))
  (bind _output_get (set `self.YawSpeed` (`KismetMathLibrary.FInterpTo` (`self.YawSpeed`) (`self.TargetYawSpeed`) DeltaSeconds 2.0)))
  (`self.K2_AddActorLocalRotation` (`KismetMathLibrary.MakeRotator` 0.0 0.0 (* _output_get DeltaSeconds))))

(event `self.ReceiveBeginPlay`
  (bind _returnvalue (`InputDeviceLibrary.GetPlayerControllerFromInputDevice` (struct)))
  (`EnhancedInputSubsystemInterface.AddMappingContext` (pcsubsystem `EnhancedInputLocalPlayerSubsystem` _returnvalue) "/Game/Input/IMC_Spaceship.IMC_Spaceship" 0 (struct))
  (bind _returnvalue_2 (`|CreateWidget` "/Game/BluePrints/WBP_InteractionHint.WBP_InteractionHint_C"))
  (`UserWidget.AddToViewport` _returnvalue_2 0))

(event `self.CockpitTrigger.OnComponentBeginOverlap`
  (params (OverlappedComponent :type "PrimitiveComponent Object Reference") (OtherActor :type "Actor Object Reference") (OtherComp :type "PrimitiveComponent Object Reference") (OtherBodyIndex :type Integer) (bFromSweep :type Boolean) (SweepResult :type "HitResult Structure (by ref)"))
  (bind _returnvalue (`InputDeviceLibrary.GetPlayerControllerFromInputDevice` (struct)))
  (`Controller.Possess` _returnvalue self))

(event `self.ReceivePossessed`
  (params (NewController :type "Controller Object Reference"))
  (bind _asplayer_controller (cast `PlayerController` NewController))
  (bind _returnvalue (pcsubsystem `EnhancedInputLocalPlayerSubsystem` _asplayer_controller))
  (`EnhancedInputSubsystemInterface.RemoveMappingContext` _returnvalue "/Game/Input/IMC_PlayerCharacter.IMC_PlayerCharacter" (struct))
  (`EnhancedInputSubsystemInterface.AddMappingContext` _returnvalue "/Game/Input/IMC_Spaceship.IMC_Spaceship" 0 (struct)))

(fn `UserConstructionScript`)